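; BP_LocationMove is a dev test actor that moves a Cone and a Sphere up and down in a continuous ping-pong loop.
; On BeginPlay it plays the albTimelineSimple timeline, lerping each component's relative height, the Cone on the SmoothUp track and the Sphere on LinearUp.
; When the timeline finishes, it toggles IsReverse to alternate between reverse and forward playback.
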(event EventBeginPlay
  (bind (_linearup _lineardown _smoothup) (Utilities|AlbTimelineSimple 1.0 false :!label _label)
    (:Update
      (Transformation|SetRelativeLocation (Variables|Default|GetCone) (Math|Vector|Lerp(Vector) "0, 0,90.000000" "0, 0,200.000000" _smoothup) false false)
      (Transformation|SetRelativeLocation (Variables|Default|GetSphere) (Math|Vector|Lerp(Vector) "0, 0,200.000000" "0, 0,310.000000" _linearup) false false))
    (:Finished
      (Variables|Default|SetIs%20Reverse (not (Variables|Default|GetIs%20Reverse)))
      (if (Variables|Default|GetIs%20Reverse)
        (goto _label Reverse)
        (else
          (goto _label))))))

(fn ConstructionScript)