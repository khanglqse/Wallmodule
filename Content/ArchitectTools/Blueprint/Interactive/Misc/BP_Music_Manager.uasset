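; Music manager Blueprint that plays randomly chosen tracks from a swappable music list, starting at BeginPlay if the list is filled.
; ChangeMusic stores the new list, fades out the current audio, waits, then fades in a random track.
; When audio finishes, it replays the same track if looping, otherwise picks another, excluding the stored index.
; EditVolume uses a smoothed timeline helper to ramp the volume multiplier to a target level.
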(event OnAudioFinished(CurrentAudio)
  (bind _current_audio (Variables|Default|GetCurrent%20Audio))
  (if (stale Custom|Change%20Music Is%20Loop)
    (Audio|Components|Audio|FadeIn (Variables|Default|GetCurrent%20Audio) (stale Custom|Change%20Music FadeInDuration) 1.0 0.0 :!class /Script/Engine.AudioComponent)
    (else
      (Variables|Default|SetIndex%20Music (.Index (Utilities|AlbRandomItem (Variables|Default|GetCurrent%20List%20Music) (Variables|Default|GetIndex%20Music))))
      (Audio|Components|Audio|SetSound _current_audio (.Item (Utilities|AlbRandomItem (Variables|Default|GetCurrent%20List%20Music) (Variables|Default|GetIndex%20Music))))
      (Audio|Components|Audio|FadeIn _current_audio (stale Custom|Change%20Music FadeInDuration) 1.0 0.0 :!class /Script/Engine.AudioComponent))))

(event Custom|Change%20Music
  (params (NewSound :type Array%20of%20Sound%20Base%20Object%20References) (FadeInDuration :type Float%20%28single-precision%29) (FadeOutDuration :type Float%20%28single-precision%29) (Is%20Loop :type Boolean))
  (bind _current_audio (Variables|Default|GetCurrent%20Audio))
  (Variables|Default|SetCurrent%20List%20Music NewSound)
  (Variables|Default|SetIndex%20Music -1)
  (if (!= (Variables|/Script/Engine.AudioComponent|GetSound (Variables|Default|GetCurrent%20Audio)) 0)
    (Audio|Components|Audio|FadeOut _current_audio FadeOutDuration 0.0 :!class /Script/Engine.AudioComponent)
    (Utilities|FlowControl|Delay FadeOutDuration))
  (Audio|Components|Audio|SetSound _current_audio (.Item (Utilities|AlbRandomItem (Variables|Default|GetCurrent%20List%20Music) (Variables|Default|GetIndex%20Music))))
  (Variables|Default|SetIndex%20Music (.Index (Utilities|AlbRandomItem (Variables|Default|GetCurrent%20List%20Music) (Variables|Default|GetIndex%20Music))))
  (Audio|Components|Audio|FadeIn _current_audio FadeInDuration 1.0 0.0 :!class /Script/Engine.AudioComponent))

(event Custom|Edit%20Volume
  (params (FadeVolumeLevel :type Float%20%28single-precision%29) (Edit%20In%20... :type Float%20%28single-precision%29))
  (Variables|Default|SetEdit%20Value (- FadeVolumeLevel (Variables|Default|GetCurrent%20Volume)))
  (bind _smoothup (Utilities|AlbTimelineSimple Edit%20In%20... false)
    (:Update
      (Audio|Components|Audio|SetVolumeMultiplier (Variables|Default|GetCurrent%20Audio) (+ (Variables|Default|GetCurrent%20Volume) (* (Variables|Default|GetEdit%20Value) _smoothup)) :!class /Script/Engine.AudioComponent))
    (:Finished
      (Variables|Default|SetCurrent%20Volume FadeVolumeLevel))))

(event EventBeginPlay
  (if (> (Utilities|Array|Length (Variables|Default|GetCurrent%20List%20Music)) 0)
    (CallFunction|ChangeMusic (Variables|Default|GetCurrent%20List%20Music) 2.0 2.0 true)))

(fn ConstructionScript)