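; Interactive measuring-tape actor that draws a line between two points and labels its length in cm.
; While mouse or touch is held, a looping timer traces from cursor or touch, stretching the cylinder, placing the end point and label, and snapping rotation to SnapAngle.
; On release, it clears SaveMeasure on the player's BP_Interactive_Comp and opens a Tick gate that keeps turning the label toward the camera in 90-degree steps.
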(event Custom|Draw%20Measure
  (bind _returnvalue (Game|GetPlayerController 0))
  (bind _platform (Class|ContactBP|GetInfoGameIns(Message) (Game|GetGameInstance)))
  (bind _outhit (CallFunction|LinetracebyControl (Utilities|Select :Index _platform :NewEnumerator0 (select (Variables|/Script/Engine.PlayerController|GetbShowMouseCursor (Game|GetPlayerController 0)) "NewEnumerator0" "NewEnumerator2") :NewEnumerator1 "NewEnumerator1") 1e+04 "ForOneFrame"))
  (Variables|Default|SetLocation%202 (- (.Location (Collision|BreakHitResult _outhit)) (Transformation|GetActorLocation)))
  (Variables|Default|SetLocation%201 (Transformation|GetWorldLocation (Variables|Default|GetPoint%201)))
  (CallFunction|UpdateMeasure)
  (CallFunction|UpdateText)
  (if (not (or (Game|Player|IsInputKeyDown _returnvalue "LeftMouseButton") (Game|Player|IsInputKeyDown _returnvalue "Touch1")))
    (Variables|/Game/ArchitectTools/Blueprint/BP_Interactive_Comp.BP_Interactive_Comp_C|SetSave%20Measure (Actor|GetComponentbyClass (Game|GetPlayerCharacter 0) "/Game/ArchitectTools/Blueprint/BP_Interactive_Comp.BP_Interactive_Comp_C") 0)
    (Utilities|Time|ClearandInvalidateTimerbyHandle (stale EventBeginPlay _returnvalue_2))
    (Utilities|FlowControl|Gate true) ; enters at Open
  ))

(event EventBeginPlay
  (bind _returnvalue (Game|GetPlayerController 0))
  (if (or (Game|Player|IsInputKeyDown _returnvalue "LeftMouseButton") (Game|Player|IsInputKeyDown _returnvalue "Touch1"))
    (bind _returnvalue_2 (Utilities|Time|SetTimerbyEvent (delegate Custom|Draw%20Measure) 0.001 true))
    (else
      (Utilities|FlowControl|Gate true) ; enters at Open
    )))

(event EventTick
  (params (DeltaSeconds :type Float%20%28single-precision%29))
  (Utilities|FlowControl|Gate true
    (:Exit
      (CallFunction|UpdateText))))

(fn ConstructionScript
  (CallFunction|UpdateMeasure)
  (Transformation|SetRelativeRotation (Variables|Default|GetPivot%20Text) (Math|Rotator|MakeRotator (Variables|Default|GetAngle%20Around%20Measure) 0.0 0.0) false false)
  (Transformation|SetRelativeRotation (Variables|Default|GetDimension%20Text) (Math|Rotator|MakeRotator 0.0 0.0 (Variables|Default|GetAngle%20Text)) false false))

(fn UpdateMeasure
  (bind _returnvalue (Transformation|GetActorLocation))
  (bind _point_1 (Variables|Default|GetPoint%201))
  (bind _snap_angle (Variables|Default|GetSnap%20Angle))
  (bind _location_2 (Variables|Default|GetLocation%202))
  (bind _location_2_2 (Variables|Default|GetLocation%202))
  (bind _returnvalue_2 (Math|Vector|VectorLength _location_2_2))
  (bind _returnvalue_3 (Transformation|GetWorldLocation _point_1))
  (bind _returnvalue_4 (+ _location_2 _returnvalue))
  (bind _returnvalue_5 (Math|Rotator|FindLookatRotation _returnvalue_3 _returnvalue_4))
  (bind (_roll _pitch _yaw) (Math|Rotator|BreakRotator _returnvalue_5))
  (Rendering|Components|TextRender|SetText (Variables|Default|GetDimension%20Text) (Utilities|Text|ToText(String) (Utilities|String|Append (Utilities|String|ToString(Integer) (Math|Float|Truncate (- (Math|Vector|VectorLength _location_2_2) 2.0))) " cm")))
  (Transformation|SetRelativeScale3D (Variables|Default|GetCylinder) (Math|Vector|MakeVector 0.5 0.5 (/ _returnvalue_2 2e+01)))
  (Transformation|SetRelativeLocation (Variables|Default|GetPoint%202) (Math|Vector|MakeVector (* _returnvalue_2 5.0) 0.0 0.0) false false)
  (Transformation|SetRelativeLocation (Variables|Default|GetPivot%20Text) (Math|Vector|MakeVector (* _returnvalue_2 2.5) 0.0 0.0) false false)
  (Transformation|SetWorldRotation _point_1 (Math|Rotator|MakeRotator (Math|Float|SnapToGrid(Float) _roll _snap_angle) (Math|Float|SnapToGrid(Float) _pitch _snap_angle) (Math|Float|SnapToGrid(Float) _yaw _snap_angle)) false false))

(fn UpdateText
  (bind _returnvalue (Game|GetPlayerCameraManager 0))
  (bind _pivot_text (Variables|Default|GetPivot%20Text))
  (bind _returnvalue_2 (Transformation|GetActorForwardVector _returnvalue))
  (bind _returnvalue_3 (Math|Vector|GetRightVector _pivot_text))
  (bind _returnvalue_4 (CallFunction|AlbAngle(vector) _returnvalue_2 _returnvalue_3 false))
  (bind _returnvalue_5 (* _returnvalue_4 -1.0))
  (bind _returnvalue_6 (Math|Float|SnapToGrid(Float) _returnvalue_5 9e+01))
  (if (and (Math|Float|InRange(Float) _returnvalue_6 -9e+01 9e+01) (!= _returnvalue_6 0.0))
    (Transformation|SetRelativeRotation (Variables|Default|GetDimension%20Text) (Math|Rotator|MakeRotator 0.0 0.0 _returnvalue_6) false false)))

(fn GetInfoInteractive
  (return false false))

(fn GetInfoGameIns
  (return "NewEnumerator0" 0 0 "NewEnumerator0" 0 0))

(fn GetInfoPawn
  (return 0 0 "0, 0, 0" 0.0 0.0 0.0 0.0 0.0 0 0 "0, 0, 0" 0.0 0.0 0.0 0.0 0.0))