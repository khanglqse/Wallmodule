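; BP_AutoCapture_Material is an ArchitectTools helper that renders a preview image of a material.
; Start Capture applies the material to a plane and has a scene capture component render only that plane into a new render target.
; It returns a dynamic instance of ReviewCapture_M with the captured render target set as its texture parameter.
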(fn ConstructionScript)

(fn StartCapture
  (bind _capture_scene (Variables|Default|GetCapture%20Scene))
  (Rendering|Material|SetMaterial (Variables|Default|GetCapture%20Plane) 0 (Variables|Default|GetMaterial))
  (Rendering|SceneCapture|ShowOnlyComponent (Variables|Default|GetCapture%20Scene) (Variables|Default|GetCapture%20Plane))
  (bind _returnvalue (Rendering|CreateRenderTarget2D 256 256 "RTF_RGBA16f"))
  (bind _output_get (Variables|/Script/Engine.SceneCaptureComponent2D|SetTextureTarget _capture_scene _returnvalue))
  (Rendering|SceneCapture|CaptureScene _capture_scene :!class /Script/Engine.SceneCaptureComponent2D)
  (bind _returnvalue_2 (Rendering|Material|CreateDynamicMaterialInstance "/Game/ArchitectTools/Blueprint/Interactive/EditObject/Dev/ReviewCapture_M.ReviewCapture_M" "None" :!class /Script/Engine.KismetMaterialLibrary))
  (Rendering|Material|SetTextureParameterValue _returnvalue_2 "Capture Texture" _output_get)
  (return _returnvalue_2))