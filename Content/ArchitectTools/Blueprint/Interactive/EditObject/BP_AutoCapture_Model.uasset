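; Capture actor that renders a preview image of a given static mesh or actor class and returns it as a dynamic material.
; A mesh is framed by scaling the camera arm and ortho width to its bounds; an actor class spawns as a child actor with fixed framing.
; Start Capture restricts the scene capture to that subject, renders once to a new render target and feeds it into a ReviewCapture_M instance.
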(event EventBeginPlay)

(event Collision|EventActorBeginOverlap
  (params (OtherActor :type Actor%20Object%20Reference)))

(event EventTick
  (params (DeltaSeconds :type Float%20%28single-precision%29)))

(fn ConstructionScript)

(fn NavigateLocationtoCapture
  (bind _model_capture (Variables|Default|GetModel%20Capture))
  (bind _arm_camera (Variables|Default|GetArm_Camera))
  (bind _returnvalue (StaticMesh|GetBounds _model_capture))
  (Utilities|IsValid (Variables|Default|GetModel%20Capture)
    (:Is%20Valid
      (Components|StaticMesh|SetStaticMesh (Variables|Default|GetModel) (Variables|Default|GetModel%20Capture))
      (bind _output_get (Variables|/Script/Engine.SpringArmComponent|SetTargetArmLength _arm_camera (* (.sphereradius _returnvalue) 2.2)))
      (Variables|/Script/Engine.SceneCaptureComponent2D|SetOrthoWidth (Variables|Default|GetScene%20Capture) _output_get)
      (Transformation|SetRelativeLocation _arm_camera (.origin _returnvalue) false false))
    (:Is%20Not%20Valid
      (if (!= (Variables|Default|GetActor%20capture) 0)
        (ChildActorComponent|SetChildActorClass (Variables|Default|GetActor) (Variables|Default|GetActor%20capture))
        (Rendering|SetVisibility (Variables|Default|GetModel) false false)
        (bind _output_get_2 (Variables|/Script/Engine.SpringArmComponent|SetTargetArmLength (Variables|Default|GetArm_Camera) 2.5e+02))
        (Variables|/Script/Engine.SceneCaptureComponent2D|SetOrthoWidth (Variables|Default|GetScene%20Capture) _output_get_2)))))

(fn StartCapture
  (CallFunction|NavigateLocationtoCapture)
  (Utilities|IsValid (Variables|Default|GetModel%20Capture)
    (:Is%20Valid
      (Rendering|SceneCapture|ShowOnlyComponent (Variables|Default|GetScene%20Capture) (Variables|Default|GetModel))
      (bind _returnvalue (Rendering|CreateRenderTarget2D 256 256 "RTF_RGBA16f" :!label _label))
      (bind _output_get (Variables|/Script/Engine.SceneCaptureComponent2D|SetTextureTarget (Variables|Default|GetScene%20Capture) _returnvalue))
      (Rendering|SceneCapture|CaptureScene (Variables|Default|GetScene%20Capture) :!class /Script/Engine.SceneCaptureComponent2D)
      (bind _returnvalue_2 (Rendering|Material|CreateDynamicMaterialInstance "/Game/ArchitectTools/Blueprint/Interactive/EditObject/Dev/ReviewCapture_M.ReviewCapture_M" "None" :!class /Script/Engine.KismetMaterialLibrary))
      (Rendering|Material|SetTextureParameterValue _returnvalue_2 "Capture Texture" _output_get)
      (return _returnvalue_2))
    (:Is%20Not%20Valid
      (if (!= (Variables|Default|GetActor%20capture) 0)
        (Rendering|SceneCapture|ShowOnlyActorComponents (Variables|Default|GetScene%20Capture) self)
        (goto _label)))))