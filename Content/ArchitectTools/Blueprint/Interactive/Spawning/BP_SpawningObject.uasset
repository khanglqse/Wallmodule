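; BP_SpawningObject is an actor in the ArchitectTools interactive spawning set that displays a configurable static mesh.
; UpdateModel runs from the construction script and again on BeginPlay, assigning ModelStatic to the StaticMesh component.
; It then offsets the component using the mesh bounds so the model is centered horizontally on the actor origin with its base at origin height, regardless of the mesh's own pivot.
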(event EventBeginPlay
  (CallFunction|UpdateModel))

(fn ConstructionScript
  (CallFunction|UpdateModel))

(fn UpdateModel
  (bind _model_static (Variables|Default|GetModel%20Static))
  (bind _returnvalue (StaticMesh|GetBounds _model_static))
  (bind (_origin _boxextent) (Math|BoxSphereBounds|BreakBoxSphereBounds _returnvalue))
  (Components|StaticMesh|SetStaticMesh (Variables|Default|GetStaticMesh) (Variables|Default|GetModel%20Static))
  (Transformation|SetRelativeLocation (Variables|Default|GetStaticMesh) (+ (- "0, 0, 0" _origin) (Math|Vector|MakeVector 0.0 0.0 (.Z (Math|Vector|BreakVector _boxextent)))) false false))