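; BP_AreaMinimap is a box volume that defines a minimap area and switches the player HUD's minimap as the player moves through it.
; On BeginPlay it collects overlapping BP_CameraView actors as viewer points.
; Player entry, checked after a short retriggerable delay, passes this area to the HUD minimap; exit passes ParentMinimap, allowing nested areas.
; The construction script sizes the box and an optional preview mesh showing the Minimap texture through a dynamic material.
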(event OnComponentBeginOverlap(OverlapCollision)
  (params (OverlappedComponent :type Primitive%20Component%20Object%20Reference) (OtherActor :type Actor%20Object%20Reference) (OtherComp :type Primitive%20Component%20Object%20Reference) (OtherBodyIndex :type Integer) (bFromSweep :type Boolean) (SweepResult :type Hit%20Result%20Structure%20%28by%20ref%29))
  ;[1 1 1] Update overlap
  (Utilities|Array|Add (Variables|Default|GetList%20Overlap) OtherActor)
  (Utilities|FlowControl|RetriggerableDelay 0.1)
  (if (Utilities|Array|ContainsItem (Variables|Default|GetList%20Overlap) (Game|GetPlayerCharacter 0))
    (bind _player_hud (Class|ContactBP|GetInfoGameIns(Message) (Game|GetGameInstance)))
    (Default|UpdateMinimap (Variables|/Game/ArchitectTools/Blueprint/UI_HUD.UI_HUD_C|GetBP_Minimap _player_hud) self)))

(event OnComponentEndOverlap(OverlapCollision)
  (params (OverlappedComponent :type Primitive%20Component%20Object%20Reference) (OtherActor :type Actor%20Object%20Reference) (OtherComp :type Primitive%20Component%20Object%20Reference) (OtherBodyIndex :type Integer))
  ;[1 1 1] Update overlap
  (Utilities|Array|RemoveItem (Variables|Default|GetList%20Overlap) OtherActor)
  (if (== OtherActor (Game|GetPlayerCharacter 0))
    (bind _player_hud (Class|ContactBP|GetInfoGameIns(Message) (Game|GetGameInstance)))
    (Default|UpdateMinimap (Variables|/Game/ArchitectTools/Blueprint/UI_HUD.UI_HUD_C|GetBP_Minimap _player_hud) (Variables|Default|GetParent%20Minimap))))

(event EventBeginPlay
  (for _array_element (Collision|GetOverlappingActors (Variables|Default|GetOverlapCollision) "/Game/ArchitectTools/Blueprint/Interactive/CameraView/BP_CameraView.BP_CameraView_C" :!class /Script/Engine.PrimitiveComponent)
    (bind _asbp_camera_view (Utilities|Casting|CastToBP_CameraView _array_element))
    (Utilities|Array|Add (Variables|Default|GetViewerPoint) _asbp_camera_view)))

(fn ConstructionScript
  (bind _minimap (Variables|Default|GetMinimap))
  (Utilities|FlowControl|Sequence
    (:then_0
      (Components|Box|SetBoxExtent (Variables|Default|GetOverlapCollision) (Variables|Default|GetSize%20Overlap) true)
      (Transformation|SetWorldScale3D (Variables|Default|GetPreview%20Minimap) (/ (Variables|Default|GetSize%20Overlap) "50.000000,50.000000,1.000000"))
      (Rendering|SetVisibility (Variables|Default|GetPreview%20Minimap) (Variables|Default|GetReview%20Minimap) false))
    (:then_1
      (bind _asmaterial_instance_dynamic (Utilities|Casting|CastToMaterialInstanceDynamic (Rendering|Material|GetMaterial (Variables|Default|GetPreview%20Minimap) 0))
        (:then
          (bind _returnvalue (Rendering|Material|GetTextureParameterValue _asmaterial_instance_dynamic "Minimap" :!class /Script/Engine.MaterialInstanceDynamic))
          (if (!= _returnvalue _minimap)
            (Rendering|Material|SetTextureParameterValue _asmaterial_instance_dynamic "Minimap" _minimap)
            (Rendering|Material|SetMaterial (Variables|Default|GetPreview%20Minimap) 0 _asmaterial_instance_dynamic)))
        (:CastFailed
          (bind _returnvalue_2 (Rendering|Material|CreateDynamicMaterialInstance "/Game/ArchitectTools/Material/Review_Minimap_M.Review_Minimap_M" "None" :!class /Script/Engine.KismetMaterialLibrary))
          (Rendering|Material|SetTextureParameterValue _returnvalue_2 "Minimap" (Variables|Default|GetMinimap))
          (Rendering|Material|SetMaterial (Variables|Default|GetPreview%20Minimap) 0 _returnvalue_2))))))

(fn GetInfoGameIns
  (return "NewEnumerator0" 0 0))

(fn GetInfoInteractive
  (return false))

(fn GetInfoPawn
  (return 0 0 "0, 0, 0" 0.0 0.0 0.0 0.0 0.0 0))