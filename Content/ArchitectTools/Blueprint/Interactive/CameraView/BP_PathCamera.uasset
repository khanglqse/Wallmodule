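; BP_PathCamera is a spline path actor that flies a CameraView along its curve for camera animations.
; PathAnimation runs a timeline over TimeTravel with linear, smooth or reversed easing, aiming the camera arm at an optional focus point offset from the actor.
; When finished, it triggers the next entry in the CameraView's ListPath, wrapping around, if that view is the player character.
; The construction script previews the camera at CurrentDistance, applies spline looping and resets any actor rotation with a warning.
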(event Custom|Path%20Animation
  (params (CameraView :type BP%20Camera%20View%20Object%20Reference))
  (Variables|Default|SetCameraView CameraView)
  (Variables|Default|SetCurrent%20Distance 0.0)
  (bind (_linearup _lineardown _smoothup _smoothdown) (Utilities|AlbTimelineSimple (Variables|Default|GetTime%20Travel) false)
    (:Update
      (Variables|Default|SetCurrent%20Distance (Math|Float|Lerp 0.0 (Spline|GetSplineLength (Variables|Default|GetSpline)) (Utilities|Select :Index (Variables|Default|GetType%20Animation) :NewEnumerator0 _linearup :NewEnumerator1 _smoothup :NewEnumerator2 _lineardown :NewEnumerator3 _smoothdown)))
      (Transformation|SetActorLocation (Variables|Default|GetCameraView) (Spline|GetLocationatDistanceAlongSpline (Variables|Default|GetSpline) (Variables|Default|GetCurrent%20Distance) "World") false false)
      (if (Math|Vector|NotEqual(Vector) (Variables|Default|GetForcus%20Point) "0, 0, 0" 0.0001)
        (Transformation|SetRelativeRotation (Variables|/Game/ArchitectTools/Blueprint/Interactive/CameraView/BP_CameraView.BP_CameraView_C|GetArm_Camera (Variables|Default|GetCameraView)) (Math|Rotator|FindLookatRotation (Transformation|GetWorldLocation (Variables|/Game/ArchitectTools/Blueprint/Interactive/CameraView/BP_CameraView.BP_CameraView_C|GetCamera (Variables|Default|GetCameraView))) (+ (Variables|Default|GetForcus%20Point) (Transformation|GetActorLocation))) false false)))
    (:Finished
      (if (== (Variables|Default|GetCameraView) (Game|GetPlayerCharacter 0))
        (CallFunction|PathAnimation (Utilities|Array|Get(acopy) (Variables|/Game/ArchitectTools/Blueprint/Interactive/CameraView/BP_CameraView.BP_CameraView_C|GetList%20Path (Variables|Default|GetCameraView)) (select (> (+ (Utilities|Array|FindItem (Variables|/Game/ArchitectTools/Blueprint/Interactive/CameraView/BP_CameraView.BP_CameraView_C|GetList%20Path (Variables|Default|GetCameraView)) self) 1) (Utilities|Array|LastIndex (Variables|/Game/ArchitectTools/Blueprint/Interactive/CameraView/BP_CameraView.BP_CameraView_C|GetList%20Path (Variables|Default|GetCameraView)))) 0 (+ (Utilities|Array|FindItem (Variables|/Game/ArchitectTools/Blueprint/Interactive/CameraView/BP_CameraView.BP_CameraView_C|GetList%20Path (Variables|Default|GetCameraView)) self) 1))) (Variables|Default|GetCameraView))))))

(fn ConstructionScript
  (CallFunction|UpdateTransform 0.0)
  (Variables|Default|SetCurrent%20Distance (Math|Float|Clamp(Float) (Variables|Default|GetCurrent%20Distance) 0.0 (Spline|GetSplineLength (Variables|Default|GetSpline))))
  (Spline|SetClosedLoop (Variables|Default|GetSpline) (Variables|Default|GetIs%20Loop) true))

(fn UpdateTransform
  (params (Delta%20Time :type Float%20%28single-precision%29))
  (bind _returnvalue (Transformation|GetActorLocation))
  (bind _cameraview (Variables|Default|GetCameraView))
  (bind _forcus_point (Variables|Default|GetForcus%20Point))
  (bind _camera (Variables|/Game/ArchitectTools/Blueprint/Interactive/CameraView/BP_CameraView.BP_CameraView_C|GetCamera _cameraview))
  (bind _returnvalue_2 (Transformation|GetWorldLocation _camera))
  (bind _returnvalue_3 (- _returnvalue_2 _returnvalue))
  (bind _returnvalue_4 (Math|Rotator|FindLookatRotation _returnvalue_3 _forcus_point))
  (bind (_roll _pitch _yaw) (Math|Rotator|BreakRotator _returnvalue_4))
  (Transformation|SetActorLocation (Variables|Default|GetCameraView) (Spline|GetLocationatDistanceAlongSpline (Variables|Default|GetSpline) (Variables|Default|GetCurrent%20Distance) "World") false false)
  (Utilities|FlowControl|Sequence
    (:then_0
      (if (Math|Vector|NotEqual(Vector) (Variables|Default|GetForcus%20Point) "0, 0, 0" 0.0001)
        (Transformation|SetRelativeRotation (Variables|/Game/ArchitectTools/Blueprint/Interactive/CameraView/BP_CameraView.BP_CameraView_C|GetArm_Camera _cameraview) (Math|Rotator|MakeRotator _roll _pitch (- _yaw (.Yaw (Math|Rotator|BreakRotator (Transformation|GetActorRotation (Variables|Default|GetCameraView)))))) false false)))
    (:then_1
      (if (Utilities|Enum|NotEqual(Enum) (Transformation|GetActorRotation) "0, 0, 0")
        (Transformation|SetActorRotation "0, 0, 0")
        (Development|PrintString "Please Do Not Rotate This Actor !" true true "(R=1.000000,G=0.000000,B=0.010913,A=1.000000)")))))