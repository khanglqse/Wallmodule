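; Interaction component for an architectural tool that handles object customization, measurement markers, drag-moving and spawn placement.
; Platform-aware cursor or touch line traces drive customization for data-table objects, Contact_BP interface messages, and BP_Measure spawning or removal.
; Movable actors attach to a spawned pivot, which interpolates toward the trace point through a Delay loop while pressed.
; Spawn placement uses a gated loop until broken; both modes highlight meshes with custom depth and disable collision.
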(event Custom|Call%20Move
  (params (Actor%20Move :type Actor%20Object%20Reference))
  (Utilities|SetLocationMove Actor%20Move))

(event Custom|Call%20Spawn
  (params (Actor%20Move :type Actor%20Object%20Reference))
  (Utilities|SetLocationSpawn Actor%20Move))

(event Custom|Break%20Spawn
  (Utilities|SetLocationSpawn (stale Custom|Call%20Spawn Actor%20Move)) ; enters at Break
)

(fn CallInteractive
  (bind (_platform _player_hud) (Class|ContactBP|GetInfoGameIns(Message) (Game|GetGameInstance)))
  (bind (_outhit _returnvalue) (CallFunction|LinetracebyControl (Utilities|Select :Index _platform :NewEnumerator0 (select (Variables|/Script/Engine.PlayerController|GetbShowMouseCursor (Game|GetPlayerController 0)) "NewEnumerator0" "NewEnumerator2") :NewEnumerator1 "NewEnumerator1") 1e+07 "ForDuration"))
  (if _returnvalue
    (Utilities|FlowControl|Sequence
      (:then_0
        (bind _outrownames (DataTable|GetDataTableRowNames "/Game/ArchitectTools/Blueprint/Interactive/EditObject/Dev/Customize_DATA.Customize_DATA"))
        (if (Utilities|Array|ContainsItem _outrownames (Utilities|String|StringToName (CallFunction|GetRealName (.HitActor (Collision|BreakHitResult _outhit)))))
          (Utilities|IsValid (Actor|GetComponentbyClass (.HitActor (Collision|BreakHitResult _outhit)) "/Script/Engine.StaticMeshComponent")
            (:Is%20Valid
              (Default|WidgetAnimatorPlay (Variables|/Game/ArchitectTools/Blueprint/Interactive/CameraView/Widget/UI_Camera_Control.UI_Camera_Control_C|GetWidgetAnimator (Variables|/Game/ArchitectTools/Blueprint/UI_HUD.UI_HUD_C|GetCamera_Control _player_hud)) "NewEnumerator1" 1.0)
              (Default|Customize (Variables|/Game/ArchitectTools/Blueprint/UI_HUD.UI_HUD_C|GetCustomizeObject _player_hud) (.HitActor (Collision|BreakHitResult _outhit)))))
          (else
            (Default|Customize (Variables|/Game/ArchitectTools/Blueprint/UI_HUD.UI_HUD_C|GetCustomizeObject _player_hud)))))
      (:then_1
        (if (Utilities|DoesObjectImplementInterface (.HitActor (Collision|BreakHitResult _outhit)) "/Game/ArchitectTools/Blueprint/Libary_BP/Contact_BP.Contact_BP_C")
          (Class|ContactBP|Interactive(Message) (.HitActor (Collision|BreakHitResult _outhit)))
          (elif (Utilities|Array|ContainsItem _outrownames (Utilities|String|StringToName (CallFunction|GetRealName (.HitActor (Collision|BreakHitResult _outhit)))))
            _))))))

(fn CallMeasure
  (bind _platform (Class|ContactBP|GetInfoGameIns(Message) (Game|GetGameInstance)))
  (bind _outhit (CallFunction|LinetracebyControl (Utilities|Select :Index _platform :NewEnumerator0 (select (Variables|/Script/Engine.PlayerController|GetbShowMouseCursor (Game|GetPlayerController 0)) "NewEnumerator0" "NewEnumerator2") :NewEnumerator1 "NewEnumerator1") 1e+04 "None"))
  (bind _asbp_measure (Utilities|Casting|CastToBP_Measure (.HitActor (Collision|BreakHitResult _outhit)))
    (:then
      (if (!= (Variables|/Game/ArchitectTools/Blueprint/Interactive/Misc/BP_Measure.BP_Measure_C|GetCylinder _asbp_measure) (.HitComponent (Collision|BreakHitResult _outhit)))
        (bind _returnvalue (Game|SpawnActorfromClass "/Game/ArchitectTools/Blueprint/Interactive/Misc/BP_Measure.BP_Measure_C" (Math|Conversions|ToTransform(Vector) (Transformation|GetWorldLocation (.HitComponent (Collision|BreakHitResult _outhit)))) "Undefined" 0 45.0 0))
        (Variables|Default|SetSave%20Measure _returnvalue)
        (else
          (Actor|DestroyActor _asbp_measure))))
    (:CastFailed
      (bind _returnvalue_2 (Game|SpawnActorfromClass "/Game/ArchitectTools/Blueprint/Interactive/Misc/BP_Measure.BP_Measure_C" (Math|Conversions|ToTransform(Vector) (.Location (Collision|BreakHitResult _outhit))) "Undefined" 0 45.0 0))
      (Variables|Default|SetSave%20Measure _returnvalue_2))))

(fn CallMoveObject
  (bind _platform (Class|ContactBP|GetInfoGameIns(Message) (Game|GetGameInstance)))
  (bind (_outhit _returnvalue) (CallFunction|LinetracebyControl (Utilities|Select :Index _platform :NewEnumerator0 (select (Variables|/Script/Engine.PlayerController|GetbShowMouseCursor (Game|GetPlayerController 0)) "NewEnumerator0" "NewEnumerator2") :NewEnumerator1 "NewEnumerator1") 1e+04 "None"))
  (if _returnvalue
    (Utilities|Casting|CastToBP_Measure (.HitActor (Collision|BreakHitResult _outhit))
      (:CastFailed
        (if (not (Utilities|DoesObjectImplementInterface (.HitActor (Collision|BreakHitResult _outhit)) "/Game/ArchitectTools/Blueprint/Libary_BP/Contact_BP.Contact_BP_C"))
          (if (Utilities|Enum|Equal(Enum) (Variables|/Script/Engine.SceneComponent|GetMobility (.HitComponent (Collision|BreakHitResult _outhit))) "Movable")
            (Collision|SetActorEnableCollision (.HitActor (Collision|BreakHitResult _outhit)) false)
            (bind _returnvalue_2 (Game|SpawnActorfromClass "/Game/ArchitectTools/Blueprint/Interactive/EditObject/BP_PivotMovable_Object.BP_PivotMovable_Object_C" (Math|Conversions|ToTransform(Vector) (select (or (== (Utilities|GetClass (.HitActor (Collision|BreakHitResult _outhit))) "/Script/Engine.StaticMeshActor") (== (Utilities|GetClass (.HitActor (Collision|BreakHitResult _outhit))) "/Game/ArchitectTools/Blueprint/Interactive/Spawning/BP_SpawningObject.BP_SpawningObject_C")) (Transformation|GetActorLocation (.HitActor (Collision|BreakHitResult _outhit))) (.Origin (Collision|GetComponentBounds (.HitComponent (Collision|BreakHitResult _outhit)))))) "Undefined" 0 0))
            (Transformation|AttachActorToActor (.HitActor (Collision|BreakHitResult _outhit)) _returnvalue_2 "None" "SnapToTarget" "KeepWorld" "KeepWorld" true)
            (CallFunction|CallMove (.HitActor (Collision|BreakHitResult _outhit)))))))))