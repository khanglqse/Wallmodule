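; Player character for an architectural walkthrough tool, with platform-switched PC and touch controls for looking, FOV zoom and movement.
; Look input is smoothed and scaled by FOV; double click or tap traces to the floor and glides the capsule there via MoveComponentTo.
; Gates and hold timers separate clicks, short holds and long holds into InteractiveComp interact, move-object and measure calls, cancelled by swipes.
; Moved objects rotate by wheel or second finger; keys handle deletion and menus.
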(event MoveObject(Interactive_Comp)
  (params (Actor%20Move :type Actor%20Object%20Reference))
  ;[1 1 1] Interactive
  (Utilities|FlowControl|Delay 0.1)
  (Utilities|FlowControl|Gate true) ; enters at Close
)

(event Custom|Break%20Call%20Interactive
  ;[1 1 1] Interactive
  (Utilities|FlowControl|Sequence
    (:then_0
      (Utilities|FlowControl|Gate true) ; enters at Close
    )
    (:then_1
      (Utilities|HoldKey 1.0) ; enters at Break
    )
    (:then_2
      (Utilities|FlowControl|Gate true) ; enters at Close
    )))

(event Custom|Touch%201
  (params (Location :type Vector))
  ;[1 1 1] Touch Looking
  (if (not (.bIsCurrentlyPressed (Class|PlayerController|GetInputTouchState (Game|GetPlayerController 0) "Touch2")))
    (Variables|TouchScreenValue|SetVelocity%20Touch%201 (select (Math|Vector|Equal(Vector) (Variables|TouchScreenValue|GetValue%20Touch%201) "0, 0, 0" 0.0001) "0, 0, 0" (- Location (Variables|TouchScreenValue|GetValue%20Touch%201))))
    (Variables|TouchScreenValue|SetValue%20Touch%201 Location)
    (Utilities|FlowControl|Sequence
      (:then_0
        (if (CallFunction|ConditionLooking "NewEnumerator1")
          (bind _returnvalue (Utilities|SmoothValue true (Variables|PCValue|GetX%20Value) (* (.X (Math|Vector|BreakVector (Variables|TouchScreenValue|GetVelocity%20Touch%201))) 0.05) 4.0 1e-05 :!label _label)
            (:OutputPin
              (bind _output_get (Variables|PCValue|SetX%20Value _returnvalue))
              (Pawn|Input|AddControllerYawInput (* _output_get (/ (Camera|GetFOVAngle (Game|GetPlayerCameraManager 0)) 9e+01)))))
          (else
            (goto _label Break))))
      (:then_1
        (if (CallFunction|ConditionLooking "NewEnumerator1")
          (bind _returnvalue_2 (Utilities|SmoothValue true (Variables|PCValue|GetY%20Value) (* (.Y (Math|Vector|BreakVector (Variables|TouchScreenValue|GetVelocity%20Touch%201))) 0.05) 4.0 1e-05 :!label _label_2)
            (:OutputPin
              (bind _output_get_2 (Variables|PCValue|SetY%20Value _returnvalue_2))
              (Pawn|Input|AddControllerPitchInput (* _output_get_2 (/ (Camera|GetFOVAngle (Game|GetPlayerCameraManager 0)) 9e+01)))))
          (else
            (goto _label_2 Break)))))
    (else
      (Variables|TouchScreenValue|SetValue%20Touch%201 Location)
      (Utilities|FlowControl|Sequence
        (:then_0
          (goto _label Break))
        (:then_1
          (goto _label_2 Break))))))

(event Custom|Touch%202
  (params (Location :type Vector))
  ;[1 1 1] Touch Zooming
  (Variables|TouchScreenValue|SetVelocity%20Touch%202 (select (Math|Vector|Equal(Vector) (Variables|TouchScreenValue|GetValue%20Touch%202) "0, 0, 0" 0.0001) "0, 0, 0" (- Location (Variables|TouchScreenValue|GetValue%20Touch%202))))
  (Variables|TouchScreenValue|SetValue%20Touch%202 Location)
  (Variables|Default|SetZoom%20Value (select (Math|Float|NearlyEqual(Float) (Variables|Default|GetZoom%20Save) 0.0 0.001) 0.0 (- (Math|Vector|VectorLength (- (Variables|TouchScreenValue|GetValue%20Touch%201) (Variables|TouchScreenValue|GetValue%20Touch%202))) (Variables|Default|GetZoom%20Save))))
  (Variables|Default|SetZoom%20Save (Math|Vector|VectorLength (- (Variables|TouchScreenValue|GetValue%20Touch%201) (Variables|TouchScreenValue|GetValue%20Touch%202))))
  (bind _platform (Class|ContactBP|GetInfoGameIns(Message) (Game|GetGameInstance)))
  (if (Utilities|Enum|Equal(Enum) _platform "NewEnumerator1")
    (CallFunction|ZoomCamera (* (Variables|Default|GetZoom%20Value) 0.05))))

(event Custom|Zoom%20Camera
  (params (Value%20+/- :type Float%20%28single-precision%29))
  (bind _velocity_touch_2 (Variables|TouchScreenValue|GetVelocity%20Touch%202))
  (bind (_x _y) (Math|Vector|BreakVector _velocity_touch_2))
  ;[1 1 1] Touch Zooming
  (Utilities|IsValid (Variables|/Game/ArchitectTools/Blueprint/BP_Interactive_Comp.BP_Interactive_Comp_C|GetSave%20Component (Variables|Default|GetInteractive_Comp))
    (:Is%20Valid
      (CallFunction|RotateZObject (select (> (Math|Float|Absolute(Float) _x) (Math|Float|Absolute(Float) _y)) _x _y)))
    (:Is%20Not%20Valid
      (bind _returnvalue (Utilities|SmoothValue false (Variables|Default|GetZoom%20Smooth) Value%20+/- 8.0 1e-05)
        (:OutputPin
          (bind _output_get (Variables|Default|SetZoom%20Smooth _returnvalue))
          (Camera|SetFieldOfView (Variables|Default|GetCamera) (Math|Float|Clamp(Float) (- (Camera|GetFOVAngle (Game|GetPlayerCameraManager 0)) _output_get) 1.0 9e+01)))))))

(event Custom|Rotate%20Z%20Object
  (params (Axis%20value :type Float%20%28single-precision%29))
  ;[1 1 1] Rotate Object Move TouchScreen
  (Utilities|IsValid (stale MoveObject(Interactive_Comp) Actor%20Move)
    (:Is%20Valid
      (bind _platform (Class|ContactBP|GetInfoGameIns(Message) (Game|GetGameInstance)))
      (if (Utilities|Enum|Equal(Enum) _platform "NewEnumerator1")
        (bind _returnvalue (Utilities|SmoothValue true (Variables|Default|GetZ%20Rotate%20Value) (* Axis%20value 0.2) 4.0 1e-05 :!label _label)
          (:OutputPin
            (Variables|Default|SetZ%20Rotate%20Value _returnvalue)
            (Utilities|IsValid (stale MoveObject(Interactive_Comp) Actor%20Move)
              (:Is%20Valid
                (Class|Actor|AddActorWorldRotation (Actor|GetAttachParentActor (stale MoveObject(Interactive_Comp) Actor%20Move)) (Math|Rotator|MakeRotator 0.0 0.0 _returnvalue))))))))
    (:Is%20Not%20Valid
      (goto _label Break))))

(event EventBreakSomething
  ;[1 1 1] Interactive
  (CallFunction|BreakCallInteractive)
  (CallFunction|ResetTouchPad))

(event EventBeginPlay
  (Variables|/Script/Engine.PlayerController|SetbShowMouseCursor (Game|GetPlayerController 0) true))

(event Input|ActionEvents|InputActionInteractive
  (params (Key :type Key%20Structure :default "None"))
  ;[1 1 1] Interactive
  (:Pressed
    (bind _platform (Class|ContactBP|GetInfoGameIns(Message) (Game|GetGameInstance)))
    (Utilities|FlowControl|Sequence
      (:then_0
        (switch Utilities|FlowControl|Switch|SwitchonPlatform _platform
          (:NewEnumerator0
            (if (== Key "LeftMouseButton")
              (Utilities|FlowControl|Sequence
                (:then_0
                  (Utilities|DoubleClick 0.2
                    (:Exit
                      (Utilities|FlowControl|Sequence
                        (:then_0
                          (Utilities|FlowControl|Delay 0.02)
                          (goto _label_4 Close))
                        (:then_1
                          (if (Variables|/Script/Engine.PlayerController|GetbShowMouseCursor (Game|GetPlayerController 0))
                            (Utilities|AISimpleMove)))))))
                (:then_1
                  (Utilities|HoldKey 0.15 :!label _label
                    (:Success
                      (if (Math|Boolean|ANDBoolean (Math|Float|NearlyEqual(Float) (Variables|PCValue|GetX%20Value) 0.0 0.05) (Math|Float|NearlyEqual(Float) (Variables|PCValue|GetY%20Value) 0.0 0.05) (not (Utilities|IsValid (Variables|/Game/ArchitectTools/Blueprint/BP_Interactive_Comp.BP_Interactive_Comp_C|GetSave%20Component (Variables|Default|GetInteractive_Comp)))))
                        (CallFunction|BreakCallInteractive)
                        (Default|CallMoveObject (Variables|Default|GetInteractive_Comp))))))
                (:then_2
                  (goto _label_4 Open)))))
          (:NewEnumerator1
            (if (== Key "Touch1")
              (Utilities|FlowControl|Sequence
                (:then_0
                  (Utilities|DoubleClick 0.2
                    (:Exit
                      (Utilities|FlowControl|Sequence
                        (:then_0
                          (Utilities|FlowControl|Delay 0.02)
                          (goto _label_4 Close))
                        (:then_1
                          (Utilities|AISimpleMove))))))
                (:then_1
                  (Utilities|HoldKey 0.15 :!label _label_2
                    (:Success
                      (if (Math|Boolean|ANDBoolean (Math|Float|NearlyEqual(Float) (Variables|PCValue|GetX%20Value) 0.0 0.05) (Math|Float|NearlyEqual(Float) (Variables|PCValue|GetY%20Value) 0.0 0.05) (not (Utilities|IsValid (Variables|/Game/ArchitectTools/Blueprint/BP_Interactive_Comp.BP_Interactive_Comp_C|GetSave%20Component (Variables|Default|GetInteractive_Comp)))))
                        (CallFunction|BreakCallInteractive)
                        (Default|CallMoveObject (Variables|Default|GetInteractive_Comp))))))
                (:then_2
                  (goto _label_4 Open)))))))
      (:then_1
        (goto _label_5 Open))
      (:then_2
        (Utilities|HoldKey 1.0 :!label _label_3
          (:Success
            (if (Math|Boolean|ANDBoolean (Math|Float|NearlyEqual(Float) (Variables|PCValue|GetX%20Value) 0.0 0.05) (Math|Float|NearlyEqual(Float) (Variables|PCValue|GetY%20Value) 0.0 0.05) (not (Utilities|IsValid (Variables|/Game/ArchitectTools/Blueprint/BP_Interactive_Comp.BP_Interactive_Comp_C|GetSave%20Component (Variables|Default|GetInteractive_Comp)))))
              (Default|CallMeasure (Variables|Default|GetInteractive_Comp))))))))
  (:Released
    (Utilities|FlowControl|Sequence
      (:then_0
        (switch Utilities|FlowControl|Switch|SwitchonPlatform _platform
          (:NewEnumerator0
            (if (== Key "LeftMouseButton")
              (Utilities|FlowControl|RetriggerableDelay 0.1)
              (Utilities|FlowControl|Gate true :!label _label_4
                (:Exit
                  (Default|CallInteractive (Variables|Default|GetInteractive_Comp))))))
          (:NewEnumerator1
            (if (== Key "Touch1")
              (Utilities|FlowControl|RetriggerableDelay 0.2)
              (Utilities|FlowControl|Gate true :!label _label_5
                (:Exit
                  (goto _label_4)))))))
      (:then_1
        (goto _label_3 Break))
      (:then_2
        (goto _label Break))
      (:then_3
        (goto _label_2 Break)))))

(event Input|AxisEvents|InputAxisLookX
  (params (AxisValue :type Float%20%28single-precision%29))
  ;[1 1 1] PC Looking
  (if (CallFunction|ConditionLooking "NewEnumerator0")
    (bind _returnvalue (Utilities|SmoothValue true (Variables|PCValue|GetX%20Value) AxisValue 6.0 1e-05 :!label _label)
      (:OutputPin
        (bind _output_get (Variables|PCValue|SetX%20Value _returnvalue))
        (Pawn|Input|AddControllerYawInput (* _output_get (/ (Camera|GetFOVAngle (Game|GetPlayerCameraManager 0)) 9e+01)))))
    (else
      (goto _label Break))))

(event Input|AxisEvents|InputAxisMoveSW
  (params (AxisValue :type Float%20%28single-precision%29))
  ;[1 1 1] PC Movement
  (Pawn|Input|AddMovementInput (Transformation|GetActorForwardVector) AxisValue false))

(event Input|AxisEvents|InputAxisLookY
  (params (AxisValue :type Float%20%28single-precision%29))
  ;[1 1 1] PC Looking
  (if (CallFunction|ConditionLooking "NewEnumerator0")
    (bind _returnvalue (Utilities|SmoothValue true (Variables|PCValue|GetY%20Value) AxisValue 6.0 1e-05 :!label _label)
      (:OutputPin
        (bind _output_get (Variables|PCValue|SetY%20Value _returnvalue))
        (Pawn|Input|AddControllerPitchInput (* _output_get (/ (Camera|GetFOVAngle (Game|GetPlayerCameraManager 0)) 9e+01)))))
    (else
      (goto _label Break))))

(event Input|AxisEvents|InputAxisMoveAD
  (params (AxisValue :type Float%20%28single-precision%29))
  ;[1 1 1] PC Movement
  (Pawn|Input|AddMovementInput (Transformation|GetActorRightVector) AxisValue false))

(event Input|MouseEvents|MouseWheelAxis
  (params (AxisValue :type Float%20%28single-precision%29))
  ;[1 1 1] Rotate Object Move PC
  (Utilities|IsValid (stale MoveObject(Interactive_Comp) Actor%20Move)
    (:Is%20Valid
      (bind _platform (Class|ContactBP|GetInfoGameIns(Message) (Game|GetGameInstance)))
      (if (Utilities|Enum|Equal(Enum) _platform "NewEnumerator0")
        (bind _returnvalue (Utilities|SmoothValue true (Variables|Default|GetZ%20Rotate%20Value) (* AxisValue 1e+01) 4.0 1e-05 :!label _label)
          (:OutputPin
            (Variables|Default|SetZ%20Rotate%20Value _returnvalue)
            (Utilities|IsValid (stale MoveObject(Interactive_Comp) Actor%20Move)
              (:Is%20Valid
                (Class|Actor|AddActorWorldRotation (Actor|GetAttachParentActor (stale MoveObject(Interactive_Comp) Actor%20Move)) (Math|Rotator|MakeRotator 0.0 0.0 _returnvalue))))))))
    (:Is%20Not%20Valid
      (goto _label Break))))

(event Input|MouseEvents|MouseWheelAxis
  (params (AxisValue :type Float%20%28single-precision%29))
  ;[1 1 1] PC Zoom
  (bind _platform (Class|ContactBP|GetInfoGameIns(Message) (Game|GetGameInstance)))
  (if (Utilities|Enum|Equal(Enum) _platform "NewEnumerator0")
    (CallFunction|ZoomCamera (* AxisValue 5.0))))

(event Input|KeyboardEvents|Delete
  (params (Key :type Key%20Structure :default "None"))
  (:Pressed
    (Utilities|IsValid (stale MoveObject(Interactive_Comp) Actor%20Move)
      (:Is%20Valid
        (Rendering|SetActorHiddenInGame (stale MoveObject(Interactive_Comp) Actor%20Move) true)
        (Utilities|Array|AddUnique (Variables|/Script/Engine.Actor|GetTags (stale MoveObject(Interactive_Comp) Actor%20Move)) "Destroy")
        (for _array_element (Actor|GetComponentsByClass (stale MoveObject(Interactive_Comp) Actor%20Move) "/Script/Engine.StaticMeshComponent")
          (Collision|SetCollisionEnabled _array_element "NoCollision")
          (Collision|SetCollisionResponsetoChannel _array_element "ECC_Camera" "ECR_Ignore"))))))

(event Input|KeyboardEvents|Q
  (params (Key :type Key%20Structure :default "None"))
  (:Pressed
    (bind _returnvalue (UserInterface|CreateWidget "/Game/ArchitectTools/MainMenu/UI_MainMenu.UI_MainMenu_C"))
    (UserInterface|Viewport|AddtoViewport _returnvalue 2)))

(event Input|KeyboardEvents|Escape
  (params (Key :type Key%20Structure :default "None"))
  (:Pressed
    (bind _returnvalue (UserInterface|CreateWidget "/Game/ArchitectTools/MainMenu/UI_MainMenu.UI_MainMenu_C"))
    (UserInterface|Viewport|AddtoViewport _returnvalue 2)))

(event Input|KeyboardEvents|Tab
  (params (Key :type Key%20Structure :default "None"))
  (:Pressed
    (bind _player_hud (Class|ContactBP|GetInfoGameIns(Message) (Game|GetGameInstance)))
    (Default|BackButtonManager _player_hud)))

(event Input|TouchEvents|InputTouch
  (params (Location :type Vector) (FingerIndex :type ETouchIndex%20Enum))
  ;[1 1 1] Touch Control
  (:Pressed
    (CallFunction|TouchPress Location FingerIndex))
  (:Released
    (CallFunction|TouchRelease Location FingerIndex))
  (:Moved
    (CallFunction|TouchMove Location FingerIndex)))

(fn ConstructionScript)

(fn ConditionLooking
  (params (Platform :type Platform%20Enum :default "NewEnumerator0"))
  (bind _interactive_comp (Variables|Default|GetInteractive_Comp))
  (bind _platform (Class|ContactBP|GetInfoGameIns(Message) (Game|GetGameInstance)))
  (return (Math|Boolean|ANDBoolean (Utilities|Enum|Equal(Enum) _platform Platform) (or (not (Utilities|IsValid (Variables|/Game/ArchitectTools/Blueprint/BP_Interactive_Comp.BP_Interactive_Comp_C|GetSave%20Component _interactive_comp))) (and (Utilities|Enum|Equal(Enum) _platform "NewEnumerator0") (not (Variables|/Script/Engine.PlayerController|GetbShowMouseCursor (Game|GetPlayerController 0))))) (or (and (Utilities|Enum|Equal(Enum) _platform "NewEnumerator0") (not (Variables|/Script/Engine.PlayerController|GetbShowMouseCursor (Game|GetPlayerController 0)))) (not (Utilities|IsValid (Variables|/Game/ArchitectTools/Blueprint/BP_Interactive_Comp.BP_Interactive_Comp_C|GetSave%20Measure _interactive_comp)))))))

(fn ResetTouchPad
  (Variables|TouchScreenValue|SetVelocity%20Touch%201 "0, 0, 0")
  (Variables|TouchScreenValue|SetValue%20Touch%201 "0, 0, 0")
  (Variables|TouchScreenValue|SetVelocity%20Touch%202 "0, 0, 0")
  (Variables|TouchScreenValue|SetValue%20Touch%202 "0, 0, 0")
  (Variables|Default|SetZoom%20Value 0.0)
  (Variables|Default|SetZoom%20Save 0.0))

(fn TouchPress
  (params (Location :type Vector) (Finger%20Index :type ETouchIndex%20Enum :default "Touch1")))

(fn TouchRelease
  (params (Location :type Vector) (Finger%20Index :type ETouchIndex%20Enum :default "Touch1"))
  (CallFunction|ResetTouchPad)
  (if (Math|Vector|NotEqual(Vector) (Variables|TouchScreenValue|GetVelocity%20Touch%202) "0, 0, 0" 1.0)
    (CallFunction|BreakCallInteractive)))

(fn TouchMove
  (params (Location :type Vector) (Finger%20Index :type ETouchIndex%20Enum :default "Touch1"))
  (switch Utilities|FlowControl|Switch|SwitchonETouchIndex Finger%20Index
    (:Touch1
      (CallFunction|Touch1 Location)
      ;[1 1 1] Break Interactive If swipe finger
      (if (Math|Vector|NotEqual(Vector) (Variables|TouchScreenValue|GetVelocity%20Touch%201) "0, 0, 0" 0.3)
        (CallFunction|BreakCallInteractive)))
    (:Touch2
      (CallFunction|Touch2 Location)
      ;[1 1 1] Break Interactive If Touch 2
      (CallFunction|BreakCallInteractive))))

(fn GetInfoGameIns
  (return "NewEnumerator0" 0 0))

(fn GetInfoInteractive
  (return false))

(fn GetInfoPawn
  (return (Variables|Default|GetArm_Camera) (Variables|Default|GetCamera) (Transformation|GetWorldRotation (Variables|Default|GetArm_Camera)) -89.900002 89.900002 0.0 359.998993 1.0 (Variables|Default|GetInteractive_Comp)))