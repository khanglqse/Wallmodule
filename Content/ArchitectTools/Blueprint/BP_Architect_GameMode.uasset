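; Game mode for Architect Tools that sets up the HUD and saves and loads player customization of the level.
; BeginPlay collects spawnable classes from a DataTable, then tags customizable actors with their current location as an identity key.
; SaveGame records meshes, materials, colors, transforms, destroyed flags, measurements and spawned objects into BP_Customize_Save.
; LoadGame matches tagged actors by that location, reapplies their state and respawns saved objects.
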(event Custom|Mark%20Actor%20Customize
  ;[1 1 1] Mark All StaticMesh/Datasmith can Customize
  (Utilities|Array|Clear (Variables|Default|GetList%20Actor%20Customize))
  (Utilities|FlowControl|Delay 0.2)
  (bind _outactors (Actor|GetAllActorsOfClass "/Script/Engine.Actor"))
  (for _array_element _outactors
    (if (not (Utilities|DoesObjectImplementInterface _array_element "/Game/ArchitectTools/Blueprint/Libary_BP/Contact_BP.Contact_BP_C"))
      (if (Utilities|Array|ContainsItem (Variables|Default|GetOther%20Class%20Save) (Utilities|GetClass _array_element))
        (if (not (Variables|/Script/Engine.Actor|GetbHidden _array_element))
          (Utilities|Array|Add (Variables|Default|GetList%20Actor%20Customize) _array_element :!label _label))
        (else
          (Utilities|IsValid (Actor|GetComponentbyClass _array_element "/Script/Engine.StaticMeshComponent")
            (:Is%20Valid
              (if (Utilities|Enum|Equal(Enum) (Variables|/Script/Engine.SceneComponent|GetMobility (Actor|GetComponentbyClass _array_element "/Script/Engine.StaticMeshComponent")) "Movable")
                (goto _label)
                (else
                  (bind _outrownames (DataTable|GetDataTableRowNames "/Game/ArchitectTools/Blueprint/Interactive/EditObject/Dev/Customize_DATA.Customize_DATA"))
                  (if (Utilities|Array|ContainsItem _outrownames (Utilities|String|StringToName (CallFunction|GetRealName _array_element)))
                    (Utilities|Array|Add (Variables|Default|GetList%20Actor%20Customize) _array_element))))))))))
  (for _array_element_2 (Variables|Default|GetList%20Actor%20Customize)
    (Utilities|Array|Add (Variables|/Script/Engine.Actor|GetTags _array_element_2) "Save_ArchitectTools") ; Create Mark
    (Utilities|Array|Add (Variables|/Script/Engine.Actor|GetTags _array_element_2) (Utilities|String|StringToName (Utilities|String|ToString(Vector) (Transformation|GetActorLocation _array_element_2))))))

(event Custom|Save%20Game
  (params (Save%20Name :type String) (SlotName :type String))
  (CallFunction|MarkActorCustomize)
  (Utilities|FlowControl|Delay 0.2)
  (bind _returnvalue (SaveGame|DoesSaveGameExist SlotName))
  (if _returnvalue
    (bind _returnvalue_2 (SaveGame|LoadGamefromSlot SlotName))
    (bind _asbp_customize_save (Utilities|Casting|CastToBP_Customize_Save _returnvalue_2))
    (CallFunction|SaveProgress _asbp_customize_save Save%20Name SlotName)
    (else
      (bind _returnvalue_3 (SaveGame|CreateSaveGameObject "/Game/ArchitectTools/Blueprint/Interactive/EditObject/Dev/BP_Customize_Save.BP_Customize_Save_C"))
      (CallFunction|SaveProgress _returnvalue_3 Save%20Name SlotName))))

(event Custom|Save%20Progress
  (params (Save%20Object :type BP%20Customize%20Save%20Object%20Reference) (Save%20Name :type String) (SlotName :type String))
  (bind _returnvalue (Math|DateTime|Now))
  (bind (_year _month _day) (Math|DateTime|BreakDateTime _returnvalue))
  (bind _returnvalue_2 (Utilities|String|ToString(Integer) _month))
  (bind _returnvalue_3 (Utilities|String|ToString(Integer) _day))
  (bind _returnvalue_4 (Game|GetCurrentLevelName true))
  (Variables|/Game/ArchitectTools/Blueprint/Interactive/EditObject/Dev/BP_Customize_Save.BP_Customize_Save_C|SetLevel%20Name Save%20Object _returnvalue_4)
  (Variables|/Game/ArchitectTools/Blueprint/Interactive/EditObject/Dev/BP_Customize_Save.BP_Customize_Save_C|SetDate%20Save Save%20Object (Utilities|String|Append (select (> _day 9) _returnvalue_3 (Utilities|String|Append "0" _returnvalue_3)) "/" (select (> _month 9) _returnvalue_2 (Utilities|String|Append "0" _returnvalue_2)) "/" (Utilities|String|ToString(Integer) _year)))
  (Variables|/Game/ArchitectTools/Blueprint/Interactive/EditObject/Dev/BP_Customize_Save.BP_Customize_Save_C|SetSave%20Name Save%20Object Save%20Name)
  (Utilities|Map|Clear (Variables|/Game/ArchitectTools/Blueprint/Interactive/EditObject/Dev/BP_Customize_Save.BP_Customize_Save_C|GetMeasure Save%20Object))
  (Utilities|Array|Clear (Variables|/Game/ArchitectTools/Blueprint/Interactive/EditObject/Dev/BP_Customize_Save.BP_Customize_Save_C|GetRotate%20Spawning Save%20Object))
  (Utilities|Array|Clear (Variables|/Game/ArchitectTools/Blueprint/Interactive/EditObject/Dev/BP_Customize_Save.BP_Customize_Save_C|GetCustomize%20Structure Save%20Object))
  (Utilities|Map|Clear (Variables|/Game/ArchitectTools/Blueprint/Interactive/EditObject/Dev/BP_Customize_Save.BP_Customize_Save_C|GetSpawning Save%20Object))
  (for _array_element (Variables|Default|GetList%20Actor%20Customize)
    (if (Utilities|Array|ContainsItem (Variables|Default|GetOther%20Class%20Save) (Utilities|GetClass _array_element))
      (Utilities|Array|Add (Variables|/Game/ArchitectTools/Blueprint/Interactive/EditObject/Dev/BP_Customize_Save.BP_Customize_Save_C|GetOther%20Class Save%20Object) (Utilities|GetClass _array_element))
      (Utilities|Array|Add (Variables|/Game/ArchitectTools/Blueprint/Interactive/EditObject/Dev/BP_Customize_Save.BP_Customize_Save_C|GetOther%20Transform Save%20Object) (Transformation|GetActorTransform _array_element))
      (elif (not (Utilities|DoesObjectImplementInterface _array_element "/Game/ArchitectTools/Blueprint/Libary_BP/Contact_BP.Contact_BP_C"))
        (bind _asbp_measure (Utilities|Casting|CastToBP_Measure _array_element)
          (:then
            (Utilities|Map|Add (Variables|/Game/ArchitectTools/Blueprint/Interactive/EditObject/Dev/BP_Customize_Save.BP_Customize_Save_C|GetMeasure Save%20Object) (Transformation|GetActorLocation _asbp_measure) (Variables|/Game/ArchitectTools/Blueprint/Interactive/Misc/BP_Measure.BP_Measure_C|GetLocation%202 _asbp_measure)))
          (:CastFailed
            (Utilities|Array|Clear (Variables|Default|GetList%20Material))
            (Utilities|IsValid (Actor|GetComponentbyClass _array_element "/Script/Engine.StaticMeshComponent")
              (:Is%20Valid
                (for (_array_element_2 _array_index) (Rendering|Material|GetMaterials (Actor|GetComponentbyClass _array_element "/Script/Engine.StaticMeshComponent"))
                  (bind _returnvalue_5 (Rendering|Material|GetBaseMaterial _array_element_2))
                  (bind _asmaterial_instance_dynamic (Utilities|Casting|CastToMaterialInstanceDynamic _array_element_2)
                    (:then
                      (bind _returnvalue_6 (Rendering|Material|GetVectorParameterValue _asmaterial_instance_dynamic "Color" :!class /Script/Engine.MaterialInstanceDynamic)))
                    (:CastFailed
                      _))
                  (Utilities|Array|Add (Variables|Default|GetList%20Material) (Utilities|Struct|MakeSaveMaterial_Structure _array_index _returnvalue_5 _returnvalue_6)))
                (Utilities|Array|Add (Variables|/Game/ArchitectTools/Blueprint/Interactive/EditObject/Dev/BP_Customize_Save.BP_Customize_Save_C|GetCustomize%20Structure Save%20Object) (Utilities|Struct|MakeSaveCustomize_Structure (.OutConvertedVector (Math|Conversions|ToVector(Float) (Utilities|String|ToString(Name) (Utilities|Array|Get(acopy) (Variables|/Script/Engine.Actor|GetTags _array_element) (+ (Utilities|Array|FindItem (Variables|/Script/Engine.Actor|GetTags _array_element) "Save_ArchitectTools") 1))))) (Variables|/Script/Engine.StaticMeshComponent|GetStaticMesh (Actor|GetComponentbyClass _array_element "/Script/Engine.StaticMeshComponent")) (Variables|Default|GetList%20Material) (Transformation|GetWorldTransform (Actor|GetComponentbyClass _array_element "/Script/Engine.StaticMeshComponent")) (Utilities|Array|ContainsItem (Variables|/Script/Engine.Actor|GetTags _array_element) "Destroy"))))))))))
  (bind _outactors (Actor|GetAllActorsOfClass "/Game/ArchitectTools/Blueprint/Interactive/Spawning/BP_SpawningObject.BP_SpawningObject_C"))
  (for _array_element_3 _outactors
    (if (Variables|/Game/ArchitectTools/Blueprint/Interactive/Spawning/BP_SpawningObject.BP_SpawningObject_C|GetSpawning%20In%20Runtime _array_element_3)
      (Utilities|Map|Add (Variables|/Game/ArchitectTools/Blueprint/Interactive/EditObject/Dev/BP_Customize_Save.BP_Customize_Save_C|GetSpawning Save%20Object) (Transformation|GetActorLocation _array_element_3) (Variables|/Game/ArchitectTools/Blueprint/Interactive/Spawning/BP_SpawningObject.BP_SpawningObject_C|GetModel%20Static _array_element_3))
      (Utilities|Array|Add (Variables|/Game/ArchitectTools/Blueprint/Interactive/EditObject/Dev/BP_Customize_Save.BP_Customize_Save_C|GetRotate%20Spawning Save%20Object) (Transformation|GetActorRotation _array_element_3))))
  (SaveGame|SaveGametoSlot Save%20Object SlotName))

(event Custom|Load%20Game
  (params (SlotName :type String))
  (bind _returnvalue (SaveGame|LoadGamefromSlot SlotName))
  (bind _asbp_customize_save (Utilities|Casting|CastToBP_Customize_Save _returnvalue))
  (for _array_element (Variables|/Game/ArchitectTools/Blueprint/Interactive/EditObject/Dev/BP_Customize_Save.BP_Customize_Save_C|GetCustomize%20Structure _asbp_customize_save)
    (bind _outactors (Actor|GetAllActorswithTag "Save_ArchitectTools"))
    (for _array_element_2 _outactors
      (Utilities|IsValid (Actor|GetComponentbyClass _array_element_2 "/Script/Engine.StaticMeshComponent")
        (:Is%20Valid
          (if (Math|Vector|Equal(Vector) (.OutConvertedVector (Math|Conversions|ToVector(Float) (Utilities|String|ToString(Name) (Utilities|Array|Get(acopy) (Variables|/Script/Engine.Actor|GetTags _array_element_2) (+ (Utilities|Array|FindItem (Variables|/Script/Engine.Actor|GetTags _array_element_2) "Save_ArchitectTools") 1))))) (.DetectObjectbyBasicLocation (Utilities|Struct|BreakSaveCustomize_Structure _array_element)) 1e+01)
            (Components|StaticMesh|SetStaticMesh (Actor|GetComponentbyClass _array_element_2 "/Script/Engine.StaticMeshComponent") (.StaticMesh (Utilities|Struct|BreakSaveCustomize_Structure _array_element)))
            (Transformation|SetWorldTransform (Actor|GetComponentbyClass _array_element_2 "/Script/Engine.StaticMeshComponent") (.NewTransform (Utilities|Struct|BreakSaveCustomize_Structure _array_element)) false false)
            (for _array_element_3 (.Material (Utilities|Struct|BreakSaveCustomize_Structure _array_element))
              (bind _returnvalue_2 (Rendering|Material|CreateDynamicMaterialInstance (.Material (Utilities|Struct|BreakSaveMaterial_Structure _array_element_3)) "None" :!class /Script/Engine.KismetMaterialLibrary))
              (Rendering|Material|SetVectorParameterValue _returnvalue_2 "Color" (.Color (Utilities|Struct|BreakSaveMaterial_Structure _array_element_3)) :!class /Script/Engine.MaterialInstanceDynamic)
              (Rendering|Material|SetMaterial (Actor|GetComponentbyClass _array_element_2 "/Script/Engine.StaticMeshComponent") (.IndexElement (Utilities|Struct|BreakSaveMaterial_Structure _array_element_3)) _returnvalue_2)
              (Rendering|SetActorHiddenInGame _array_element_2 (.IsDestroy (Utilities|Struct|BreakSaveCustomize_Structure _array_element)))
              (Collision|SetActorEnableCollision _array_element_2 (not (.IsDestroy (Utilities|Struct|BreakSaveCustomize_Structure _array_element))))))))))
  (bind _keys (Utilities|Map|Keys (Variables|/Game/ArchitectTools/Blueprint/Interactive/EditObject/Dev/BP_Customize_Save.BP_Customize_Save_C|GetMeasure _asbp_customize_save)))
  (bind _values (Utilities|Map|Values (Variables|/Game/ArchitectTools/Blueprint/Interactive/EditObject/Dev/BP_Customize_Save.BP_Customize_Save_C|GetMeasure _asbp_customize_save)))
  (for (_array_element_4 _array_index) _keys
    (bind _returnvalue_3 (Game|SpawnActorfromClass "/Game/ArchitectTools/Blueprint/Interactive/Misc/BP_Measure.BP_Measure_C" (Math|Conversions|ToTransform(Vector) _array_element_4) "Undefined" 0 45.0 0))
    (Variables|/Game/ArchitectTools/Blueprint/Interactive/Misc/BP_Measure.BP_Measure_C|SetLocation%202 _returnvalue_3 (Utilities|Array|Get(acopy) _values _array_index))
    (Default|UpdateMeasure _returnvalue_3)
    (Default|UpdateText _returnvalue_3))
  (bind _outactors_2 (Actor|GetAllActorsOfClass "/Game/ArchitectTools/Blueprint/Interactive/Spawning/BP_SpawningObject.BP_SpawningObject_C"))
  (for _array_element_5 _outactors_2
    (if (Variables|/Game/ArchitectTools/Blueprint/Interactive/Spawning/BP_SpawningObject.BP_SpawningObject_C|GetSpawning%20In%20Runtime _array_element_5)
      (Actor|DestroyActor _array_element_5)))
  (for _array_element_6 (Variables|Default|GetOther%20Class%20Save)
    (bind _outactors_3 (Actor|GetAllActorsOfClass _array_element_6))
    (for _array_element_7 _outactors_3
      (Actor|DestroyActor _array_element_7)))
  (bind _keys_2 (Utilities|Map|Keys (Variables|/Game/ArchitectTools/Blueprint/Interactive/EditObject/Dev/BP_Customize_Save.BP_Customize_Save_C|GetSpawning _asbp_customize_save)))
  (bind _values_2 (Utilities|Map|Values (Variables|/Game/ArchitectTools/Blueprint/Interactive/EditObject/Dev/BP_Customize_Save.BP_Customize_Save_C|GetSpawning _asbp_customize_save)))
  (for (_array_element_8 _array_index_2) _keys_2
    (Game|SpawnActorfromClass "/Game/ArchitectTools/Blueprint/Interactive/Spawning/BP_SpawningObject.BP_SpawningObject_C" (Math|Transform|MakeTransform _array_element_8 (Utilities|Array|Get(acopy) (Variables|/Game/ArchitectTools/Blueprint/Interactive/EditObject/Dev/BP_Customize_Save.BP_Customize_Save_C|GetRotate%20Spawning _asbp_customize_save) _array_index_2)) "Undefined" 0 (Utilities|Array|Get(acopy) _values_2 _array_index_2) true 0))
  (for (_array_element_9 _array_index_3) (Variables|/Game/ArchitectTools/Blueprint/Interactive/EditObject/Dev/BP_Customize_Save.BP_Customize_Save_C|GetOther%20Class _asbp_customize_save)
    (Game|SpawnActorfromClass _array_element_9 (Utilities|Array|Get(acopy) (Variables|/Game/ArchitectTools/Blueprint/Interactive/EditObject/Dev/BP_Customize_Save.BP_Customize_Save_C|GetOther%20Transform _asbp_customize_save) _array_index_3) "Undefined" 0 0)))

(event EventBeginPlay
  (Utilities|FlowControl|Sequence
    (:then_0
      (bind _returnvalue (UserInterface|CreateWidget "/Game/ArchitectTools/Blueprint/UI_HUD.UI_HUD_C"))
      (bind _output_get (Variables|Default|SetHUD _returnvalue))
      (UserInterface|Viewport|AddtoViewport _output_get 0)
      ;[1 1 1] Send HUD to GameInstance
      (bind _asbp_architect_instance_game (Utilities|Casting|CastToBP_Architect_InstanceGame (Game|GetGameInstance)))
      (Variables|/Game/ArchitectTools/Blueprint/BP_Architect_InstanceGame.BP_Architect_InstanceGame_C|SetHUD _asbp_architect_instance_game (Variables|Default|GetHUD)))
    (:then_1
      (bind _asbp_architect_instance_game_2 (Utilities|Casting|CastToBP_Architect_InstanceGame (Game|GetGameInstance)))
      (bind _outactors (Actor|GetAllActorsOfClass "/Game/ArchitectTools/Blueprint/Interactive/Misc/BP_Music_Manager.BP_Music_Manager_C"))
      (Utilities|IsValid (Utilities|Array|Get(acopy) _outactors)
        (:Is%20Valid
          (Variables|/Game/ArchitectTools/Blueprint/BP_Architect_InstanceGame.BP_Architect_InstanceGame_C|SetMusic%20Manager _asbp_architect_instance_game_2 (Utilities|Array|Get(acopy) _outactors)))))
    (:then_2
      (bind _outrownames (DataTable|GetDataTableRowNames "/Game/ArchitectTools/Blueprint/Interactive/Spawning/Dev/Spawning_DATA.Spawning_DATA"))
      (for _array_element _outrownames
        (bind _returnvalue_2 (Utilities|GetDataTableRow "/Game/ArchitectTools/Blueprint/Interactive/Spawning/Dev/Spawning_DATA.Spawning_DATA" _array_element)
          (:then
            (if (!= (.ActorSpawning (Utilities|Struct|BreakSpawning_Structure _returnvalue_2)) 0)
              (Utilities|Array|AddUnique (Variables|Default|GetOther%20Class%20Save) (.ActorSpawning (Utilities|Struct|BreakSpawning_Structure _returnvalue_2))))))))
    (:then_3
      (CallFunction|MarkActorCustomize))))

(fn ConstructionScript)